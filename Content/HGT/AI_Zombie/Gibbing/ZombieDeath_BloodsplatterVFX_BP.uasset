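; Blood splatter VFX actor for zombie deaths, built on a Niagara component that appears to project a decal.
; The construction script randomises the decal's width and height within a min/max size range at a fixed depth.
; When the actor is destroyed, it tells the GameplayGM game mode once to lower the zombie death blood VFX count.
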(event Custom|UpdateDecalNumbers
  (params (DestroyedActor :type Actor%20Object%20Reference))
  (Utilities|FlowControl|DoOnce false
    (:Completed
      (bind _asgameplay_gm (Utilities|Casting|CastToGameplayGM (Game|GetGameMode)))
      (Default|UpdateZombieDeathBloodVFXCount _asgameplay_gm false))))

(event EventBeginPlay
  (Game|BindEventtoOnDestroyed (delegate Custom|UpdateDecalNumbers)))

(fn ConstructionScript
  (bind _decalminsize (Variables|Default|GetDecalMinSize))
  (bind _decalmaxsize (Variables|Default|GetDecalMaxSize))
  (bind _returnvalue (Math|Random|RandomFloatinRange _decalminsize _decalmaxsize))
  (Transformation|SetWorldScale3D (Variables|Default|GetNiagara) (Math|Vector|MakeVector 0.2 _returnvalue _returnvalue)) ; X is decal height\nY and Z are the size of decal box
)