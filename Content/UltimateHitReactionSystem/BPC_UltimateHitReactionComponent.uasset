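; Actor component that plays replicated directional hit and death reactions on a registered skeletal mesh, via server-to-multicast events.
; Hit direction, bone-mapped position and strength, which can escalate with consecutive hits, feed a Chooser Table that selects the montage.
; Motion Warping sets knockback targets, while Physics Control briefly simulates the body with an impulse, keeping feet static and fading blend weight.
; Montage notifies gate interruptions and save the death pose snapshot.
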(event Custom|SERVER_PerformHitReaction
  (params (HitCauser :type Actor%20Object%20Reference) (HitResult :type Hit%20Result%20Structure) (HitStrength :type E_HitStrength%20Enum :default "NewEnumerator0") (CauseDeath :type Boolean) (UseHitCauserDirection :type Boolean))
  ;[0.15 0.15 0.15 0.5] PerformHitReaction
  (CallFunction|MULTICASTPerformHitReaction HitCauser HitResult HitStrength CauseDeath UseHitCauserDirection))

(event Custom|PerformHitReation
  (params (HitCauser :type Actor%20Object%20Reference) (HitResult :type Hit%20Result%20Structure) (HitStrength :type E_HitStrength%20Enum :default "NewEnumerator0") (CauseDeath :type Boolean) (UseHitCauserDirection :type Boolean))
  ;[0.15 0.15 0.15 0.5] PerformHitReaction
  (CallFunction|SERVERPerformHitReaction HitCauser HitResult HitStrength CauseDeath UseHitCauserDirection))

(event Custom|MULTICAST_PerformHitReaction
  (params (HitCauser :type Actor%20Object%20Reference) (HitResult :type Hit%20Result%20Structure) (HitStrength :type E_HitStrength%20Enum :default "NewEnumerator0") (CauseDeath :type Boolean) (UseHitCauserDirection :type Boolean))
  ;[0.15 0.15 0.15 0.5] PerformHitReaction
  (bind _returnvalue (CallFunction|StartHitReaction HitCauser HitResult HitStrength CauseDeath UseHitCauserDirection))
  (Utilities|FlowControl|Sequence
    (:then_0
      (Utilities|PerformMontage _returnvalue))
    (:then_1
      (Utilities|PerformPhysicsReaction))))

(event EventBeginPlay
  (bind _returnvalue (Components|GetOwner))
  (bind _returnvalue_2 (Components|GetOwner))
  (bind _returnvalue_3 (Actor|GetComponentbyClass _returnvalue "/Script/PhysicsControl.PhysicsControlComponent"))
  (bind _returnvalue_4 (Actor|GetComponentbyClass _returnvalue_2 "/Script/MotionWarping.MotionWarpingComponent"))
  (Utilities|FlowControl|Sequence
    (:then_0
      (if (Variables|HitReactionSettings|MotionWarping|GetEnableMotionWarping)
        ;[0.15 0.15 0.15 0.5] Motion Warping
        (Utilities|IsValid _returnvalue_4
          (:Is%20Valid
            (Variables|Default|SetMotionWaringComp _returnvalue_4))
          (:Is%20Not%20Valid
            (bind _returnvalue_5 (Game|AddComponentbyClass (Components|GetOwner) "/Script/MotionWarping.MotionWarpingComponent"))
            (Variables|Default|SetMotionWaringComp _returnvalue_5)))))
    (:then_1
      (if (Variables|HitReactionSettings|Physics(Experimental)|GetEnablePhysicalReaction)
        ;[0.15 0.15 0.15 0.5] Physics Control
        (Utilities|IsValid _returnvalue_3
          (:Is%20Valid
            (Variables|Default|SetPhysicsControlComp _returnvalue_3))
          (:Is%20Not%20Valid
            (bind _returnvalue_6 (Game|AddComponentbyClass (Components|GetOwner) "/Script/PhysicsControl.PhysicsControlComponent" true))
            (Variables|Default|SetPhysicsControlComp _returnvalue_6)))
        (Utilities|FlowControl|Delay 0.2)
        (Private|InitPhysicsControl)))
    (:then_2
      (Variables|HitReaction|SetCurrHitCounterDuration (Variables|HitReactionSettings|AutoUpgradeHitStrength|GetHitCounterDuration)))))

(event EventTick
  (params (DeltaSeconds :type Float%20%28single-precision%29))
  ;[0.15 0.15 0.15 0.5] Update
  (Variables|HitReaction|SetDeltaSeconds DeltaSeconds)
  (Private|UpdatePhysics)
  (Private|UpdateHitStrength))

(fn GetHitDirection
  (params (HitResult :type Hit%20Result%20Structure%20%28by%20ref%29))
  (bind (_bblockinghit _binitialoverlap _time _distance _location _impactpoint _normal _impactnormal _physmat _hitactor) (Collision|BreakHitResult HitResult))
  (if (Variables|HitReaction|GetUse%20Hit%20Causer%20Direction)
    (Utilities|IsValid (Variables|HitReaction|GetHit%20Causer)
      (:Is%20Valid
        (LocalVariables|SetImpactNormal (Math|Vector|Normalize (- (Transformation|GetActorLocation (Variables|HitReaction|GetHit%20Causer)) (Transformation|GetActorLocation _hitactor)))))
      (:Is%20Not%20Valid
        (LocalVariables|SetImpactNormal (Math|Vector|Normalize _normal) :!label _label)))
    (else
      (goto _label)))
  (bind _output_get (LocalVariables|SetForward (Math|Vector|DotProduct (LocalVariables|GetImpactNormal) (Transformation|GetActorForwardVector _hitactor))))
  (LocalVariables|SetAbsForward (Math|Float|Absolute(Float) _output_get))
  (bind _output_get_2 (LocalVariables|SetRight (Math|Vector|DotProduct (LocalVariables|GetImpactNormal) (Transformation|GetActorRightVector _hitactor))))
  (LocalVariables|SetAbsRight (Math|Float|Absolute(Float) _output_get_2))
  (bind _output_get_3 (LocalVariables|SetUp (Math|Vector|DotProduct (LocalVariables|GetImpactNormal) (Transformation|GetActorUpVector _hitactor))))
  (LocalVariables|SetAbsUp (Math|Float|Absolute(Float) _output_get_3))
  (if (and (> (LocalVariables|GetAbsForward) (LocalVariables|GetAbsRight)) (> (LocalVariables|GetAbsForward) (LocalVariables|GetAbsUp)))
    (if (> (LocalVariables|GetForward) 0.0)
      (return "NewEnumerator0")
      (else
        (return "NewEnumerator1")))
    (elif (and (> (LocalVariables|GetAbsRight) (LocalVariables|GetAbsForward)) (> (LocalVariables|GetAbsRight) (LocalVariables|GetAbsUp)))
      (if (> (LocalVariables|GetRight) 0.0)
        (return "NewEnumerator3")
        (else
          (return "NewEnumerator2")))
      (elif (> (LocalVariables|GetUp) 0.0)
        (return "NewEnumerator4")
        (else
          (return "NewEnumerator5"))))))

(fn GetHitPosition
  (params (Key :type Name%20%28by%20ref%29))
  (bind _hitposmap (Variables|HitReactionSettings|GetHitPosMap))
  (bind (_value _returnvalue) (Utilities|Map|Find _hitposmap Key))
  (if _returnvalue
    (return _value)
    (else
      (return "NewEnumerator12"))))

(fn RegistReactionMesh
  (params (MainSkeletonMesh :type Skeletal%20Mesh%20Component%20Object%20Reference))
  (bind _output_get (Variables|Default|SetMainSkeletonMesh MainSkeletonMesh))
  (bind _skeletalmeshasset (Variables|/Script/Engine.SkeletalMeshComponent|GetSkeletalMeshAsset _output_get)
    (:then
      (Variables|HitReaction|SetSkeleton (Variables|/Script/Engine.SkeletalMesh|GetSkeleton _skeletalmeshasset)))
    (:else)))

(fn Debug
  (params (HitResult :type Hit%20Result%20Structure%20%28by%20ref%29) (HitStrength :type E_HitStrength%20Enum :default "NewEnumerator0"))
  (bind (_bblockinghit _binitialoverlap _time _distance _location _impactpoint _normal _impactnormal _physmat _hitactor _hitcomponent _hitbonename _bonename _hititem _elementindex _faceindex _tracestart _traceend) (Collision|BreakHitResult HitResult))
  (bind _returnvalue (Transformation|GetWorldLocation _hitcomponent))
  ;[0.15 0.15 0.15 0.5] Hit Reaction Debug
  (if (Variables|HitReactionSettings|Debug|GetEnableDebug)
    (Rendering|Debug|DrawDebugSphere _impactpoint 5.0 10 "(R=1.000000,G=0.000000,B=0.000000,A=1.000000)" (Variables|HitReactionSettings|Debug|GetDebugDuration) 0.2)
    (Rendering|Debug|DrawDebugArrow _impactpoint (+ _impactpoint (* (Variables|HitReaction|GetHitDir) -5e+01)) 3.0 "(R=0.000000,G=1.000000,B=0.695618,A=1.000000)" (Variables|HitReactionSettings|Debug|GetDebugDuration) 1.0)
    (Rendering|Debug|DrawDebugArrow _returnvalue (+ _returnvalue (* (Class|KismetMathLibrary|VectorNormal2D (- _tracestart _traceend) 0.0001) 5e+01)) 3.0 "(R=1.000000,G=0.000000,B=0.763262,A=1.000000)" (Variables|HitReactionSettings|Debug|GetDebugDuration) 1.0)
    (Development|PrintString (Utilities|String|ToString(Text) (Utilities|Text|FormatText "BPC_UltimateHitReactionComponent Debug Log:  
Hit Strength: {HitStrength} 
Hit Direction: {HitDirection} 
Hit Position: {HitPosition}" (Utilities|String|EnumtoString HitStrength) (Utilities|String|EnumtoString (Private|GetHitDirection HitResult)) (Utilities|String|EnumtoString (Private|GetHitPosition _hitbonename)))) true true "(R=0.279968,G=0.829145,B=1.000000,A=1.000000)" (Variables|HitReactionSettings|Debug|GetDebugDuration))))

(fn UpdateMotionWarping
  (if (Variables|HitReactionSettings|MotionWarping|GetEnableMotionWarping)
    (Class|MotionWarpingComponent|AddorUpdateWarpTargetfromLocationandRotation (Variables|Default|GetMotionWaringComp) "HitReaction" (+ (Transformation|GetActorLocation (Components|GetOwner)) (* (Variables|HitReaction|GetHitDir) (.Value (Utilities|Map|Find (Variables|HitReactionSettings|MotionWarping|GetMotionWarpingDist) (Variables|HitReaction|GetCurrHitStrength))))) (Math|Rotator|FindLookatRotation (Class|KismetMathLibrary|VectorNormal2D (* (Transformation|GetActorForwardVector (Components|GetOwner)) -1.0) 0.0001) (Class|KismetMathLibrary|VectorNormal2D (* (Variables|HitReaction|GetHitDir) -1.0) 0.0001)))))

(fn UpdatePhysics
  (if (and (Variables|HitReactionSettings|Physics(Experimental)|GetEnablePhysicalReaction) (not (Utilities|Set|Contains (Variables|HitReactionSettings|Physics(Experimental)|GetDisablephysicsParts) (Variables|HitReaction|GetHit%20Position))))
    (if (Variables|HitReaction|Physics|GetStartPhysicsReaction)
      (bind _output_get (Variables|HitReaction|Physics|SetCurrPhysicsReactionDuration (+ (Variables|HitReaction|Physics|GetCurrPhysicsReactionDuration) (Variables|HitReaction|GetDeltaSeconds))))
      (if (< _output_get (Variables|HitReactionSettings|Physics(Experimental)|GetPhysicsReactionDuration))
        (Class|PhysicsControlComponent|SetBodyModifiersinSetPhysicsBlendWeight (Variables|Default|GetPhysicsControlComp) "All" (Math|Float|Clamp(Float) (- 1.0 (/ (Variables|HitReaction|Physics|GetCurrPhysicsReactionDuration) (Variables|HitReactionSettings|Physics(Experimental)|GetPhysicsReactionDuration)))))
        (else
          (Variables|HitReaction|Physics|SetStartPhysicsReaction false)
          (Class|PhysicsControlComponent|SetBodyModifiersinSetMovementType (Variables|Default|GetPhysicsControlComp) "All" "Kinematic")
          (Class|PhysicsControlComponent|SetBodyModifiersinSetMovementType (Variables|Default|GetPhysicsControlComp) "LowerBody" "Static")))
      (else
        (Variables|HitReaction|Physics|SetCurrPhysicsReactionDuration 0.0)))))

(fn UpgradeCurrHitStrength
  (bind _currhitcount (Variables|HitReaction|GetCurrHitCount))
  (bind _hitstrengthupgradehitcount (Variables|HitReactionSettings|AutoUpgradeHitStrength|GetHitStrengthUpgradeHitCount))
  (bind (_value _returnvalue) (Utilities|Map|Find _hitstrengthupgradehitcount _currhitcount))
  (if (Variables|HitReactionSettings|AutoUpgradeHitStrength|GetEnableAutoUpgradeHitStrength)
    (if _returnvalue
      (if (> (Math|Conversions|ToInteger(Byte) _value) (Math|Conversions|ToInteger(Byte) (Variables|HitReaction|GetCurrHitStrength)))
        (Variables|HitReaction|SetCurrHitStrength _value)))
    (else
      (Variables|HitReaction|SetCurrHitStrength (Variables|HitReaction|GetInput%20Hit%20Strength)))))

(fn InitPhysicsControl
  (Variables|Default|GetPhysicsControlComp
    (:then
      (Variables|Default|GetMainSkeletonMesh
        (:then
          (Utilities|FlowControl|Sequence
            (:then_0
              (Class|PhysicsControlComponent|CreateControlsfromSkeletalMeshBelow (Variables|Default|GetPhysicsControlComp) (Variables|Default|GetMainSkeletonMesh) (Variables|HitReactionSettings|GetCenterOfMassBone) false "WorldSpace" (Variables|HitReactionSettings|Physics(Experimental)|GetPhysicsControlData) "All")
              (bind _returnvalue (Class|PhysicsControlComponent|CreateBodyModifiersfromSkeletalMeshBelow (Variables|Default|GetPhysicsControlComp) (Variables|Default|GetMainSkeletonMesh) (Variables|HitReactionSettings|GetCenterOfMassBone) false "All" (Variables|HitReactionSettings|Physics(Experimental)|GetBodyModifierData)))
              (for _array_element _returnvalue
                (if (Utilities|String|Contains (Utilities|String|ToString(Name) _array_element) "foot")
                  (Class|PhysicsControlComponent|AddBodyModifierstoSet (Variables|Default|GetPhysicsControlComp) (Utilities|Array|MakeArray _array_element (Class|SkinnedMeshComponent|GetParentBone (Variables|Default|GetMainSkeletonMesh) _array_element)) "LowerBody"))))
            (:then_1
              (Class|PhysicsControlComponent|SetBodyModifiersinSetMovementType (Variables|Default|GetPhysicsControlComp) "All" "Kinematic")
              (Class|PhysicsControlComponent|SetBodyModifiersinSetMovementType (Variables|Default|GetPhysicsControlComp) "LowerBody" "Static"))))
        (:else)))
    (:else)))

(fn StartHitReaction
  (params (HitCauser :type Actor%20Object%20Reference) (Hit%20Result :type Hit%20Result%20Structure%20%28by%20ref%29) (Input%20Hit%20Strength :type E_HitStrength%20Enum :default "NewEnumerator0") (Cause%20Death :type Boolean) (UseHitCauserDirection :type Boolean))
  (Variables|HitReaction|SetHit%20Causer HitCauser)
  (Variables|HitReaction|SetUse%20Hit%20Causer%20Direction UseHitCauserDirection)
  (bind _output_get (LocalVariables|SetHitResult%28Local%29 Hit%20Result))
  (if (.bBlockingHit (Collision|BreakHitResult _output_get))
    (Variables|HitReaction|SetCurrHitCounterDuration (Variables|HitReactionSettings|AutoUpgradeHitStrength|GetHitCounterDuration))
    (Variables|HitReaction|SetInput%20Hit%20Strength Input%20Hit%20Strength)
    (Variables|HitReaction|Death|SetCause%20Death Cause%20Death)
    (if (== (Variables|HitReaction|GetCurrHitCount) 0)
      (Variables|HitReaction|SetCurrHitStrength (Variables|HitReaction|GetInput%20Hit%20Strength))
      (else
        (Private|UpgradeCurrHitStrength)))
    (Math|Integer|IncrementInt (Variables|HitReaction|GetCurrHitCount)
      (:%20%20
        (Variables|Default|GetMainSkeletonMesh
          (:then
            (Variables|HitReaction|SetHit%20Bone%20Name (.HitBoneName (Collision|BreakHitResult (LocalVariables|GetHitResult%28Local%29))))
            (Variables|HitReaction|SetHitDir (Math|Vector|Normalize (- (.TraceEnd (Collision|BreakHitResult (LocalVariables|GetHitResult%28Local%29))) (.TraceStart (Collision|BreakHitResult (LocalVariables|GetHitResult%28Local%29))))))
            (Variables|HitReaction|SetHit%20Direction (Private|GetHitDirection (LocalVariables|GetHitResult%28Local%29)))
            (Variables|HitReaction|SetHit%20Position (Private|GetHitPosition (Variables|HitReaction|GetHit%20Bone%20Name)))
            (bind _result (|EvaluateChooser2 self)
              (:execute
                (if (> (Utilities|Array|Length _result) 0)
                  _
                  (else
                    (Development|PrintString "BPC_UltimateHitReactionComponent Warning: Unable to find montage that meets the requirements, please check if the CT_HitReactionMain contains the Skeleton of the current character" true true "(R=1.000000,G=0.000000,B=0.000000,A=1.000000)")))
                (Private|Debug (LocalVariables|GetHitResult%28Local%29) (Variables|HitReaction|GetInput%20Hit%20Strength))
                (return (select (or (== (Variables|HitReaction|GetCurrHitCount) 1) (Variables|HitReaction|Death|GetCause%20Death)) (Utilities|Array|Get(acopy) _result) (.OutItem (Utilities|Array|Random _result)))))))
          (:else
            (Development|PrintString "BPC_UltimateHitReactionComponent Warning: Reaction Skeleton is not registed. Please call RegistReactionMesh() in you character blueprint at BeginPlay()" true true "(R=1.000000,G=0.000000,B=0.000000,A=1.000000)")))))))

(fn UpdateHitStrength
  ;[0.15 0.15 0.15 0.5] Auto Upgrade HitStrength
  (bind _output_get (Variables|HitReaction|SetCurrHitCounterDuration (- (Variables|HitReaction|GetCurrHitCounterDuration) (Variables|HitReaction|GetDeltaSeconds))))
  (if (<= _output_get 0.0)
    (Variables|HitReaction|SetCurrHitCount 0)
    (Variables|HitReaction|SetCurrHitStrength "NewEnumerator0")
    (Variables|HitReaction|SetPrevHitSrength "NewEnumerator0")))